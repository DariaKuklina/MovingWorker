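; Player pawn Blueprint that handles the player's movement, camera look and a Z-key action through input events.
; On BeginPlay it adds the Enhanced Input mapping context to the local player's subsystem.
; Move input is rotated by control yaw for view-relative movement, while look input drives controller yaw and pitch.
; A raw Z key press, outside the Input Actions, fires the PlayerInputZ call.
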(event `self.ReceiveBeginPlay`
  (bind _asplayer_controller (cast `PlayerController` (`self.GetController`)))
  (`EnhancedInputSubsystemInterface.AddMappingContext` (pcsubsystem `EnhancedInputLocalPlayerSubsystem` _asplayer_controller) "/Game/Player/IMC_InputController.IMC_InputController" 0 (struct)))

(event `EnhancedInput|/Game/Player/IA_Move`
  (params (ActionValue :type "Vector2D Structure") (ElapsedSeconds :type "Float (double-precision)") (TriggeredSeconds :type "Float (double-precision)") (InputAction :type "InputAction Object Reference" :default "/Game/Player/IA_Move.IA_Move"))
  (bind (_returnvalue_roll _returnvalue_pitch _returnvalue_yaw) (`KismetMathLibrary.BreakRotator` (`self.GetControlRotation`)))
  (:`Triggered`
    (`self.AddMovementInput` (`KismetMathLibrary.GreaterGreater_VectorRotator` (`KismetMathLibrary.Conv_Vector2DToVector` ActionValue) (`KismetMathLibrary.MakeRotator` 0.0 0.0 _returnvalue_yaw)))))

(event `EnhancedInput|/Game/Player/IA_Look`
  (params (ActionValue :type "Vector2D Structure") (ElapsedSeconds :type "Float (double-precision)") (TriggeredSeconds :type "Float (double-precision)") (InputAction :type "InputAction Object Reference" :default "/Game/Player/IA_Look.IA_Look"))
  (:`Triggered`
    (`|ExecutionSequence`
      (:`then_0`
        (`self.AddControllerYawInput` ActionValue_X))
      (:`then_1`
        (`self.AddControllerPitchInput` ActionValue_Y)))))

(event `Key|Z`
  (params (Key :type "Key Structure"))
  (:`Pressed`
    (`self.PlayerInputZ`)))

(fn `UserConstructionScript`)