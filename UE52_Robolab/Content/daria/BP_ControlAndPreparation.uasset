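; BP_ControlAndPreparation scripts a worker loading a component onto a cart (Telega), then starting the cart moving.
; CallDoThings chains timed attachments and AI moves: the worker takes the component in its arm socket, carries it to the cart and walks back.
; AB_Worker's States switches animation at each stage, and CalculateInclineAngle sets its lean from spine-to-cart height before placement.
; Finally, it calls CallTelegaStartMove on the BP_Telega found in the level.
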(event `/Game/daria/BPI_Callable.CallDoThings`
  (bind _asab_worker (cast `/Game/daria/AB_Worker` (`SkeletalMeshComponent.GetAnimInstance` (`Character.Mesh` (`self.Worker`)))))
  (set `/Game/daria/AB_Worker.States` 1 _asab_worker)
  (`KismetSystemLibrary.Delay` 0.5)
  (`self.K2_AttachToComponent` (`self.Component`) (`Character.Mesh` (`self.Worker`)) "rArm_Socket" "SnapToTarget" "SnapToTarget" "KeepRelative" true)
  (`KismetSystemLibrary.Delay` 0.5)
  (set `/Game/daria/AB_Worker.States` 2 _asab_worker)
  (`|AIMoveTo` (`self.Worker`) (`SceneComponent.K2_GetComponentLocation` (`self.WalkToPoint`)) null
    (:`OnSuccess`
      (`self.CalculateInclineAngle`)
      (set `/Game/daria/AB_Worker.States` 3 _asab_worker)
      (`KismetSystemLibrary.Delay` 0.5)
      (`SceneComponent.K2_DetachFromComponent` (`Actor.RootComponent` (`self.Component`)) "KeepRelative" "KeepRelative" "KeepRelative" true)
      (`self.K2_AttachToComponent` (`self.Component`) (`/Game/daria/BP_Telega.Telega` (`self.Telega`)) "Telega_Socket" "SnapToTarget" "SnapToTarget" "KeepRelative" true)
      (`KismetSystemLibrary.Delay` 0.5)
      (set `/Game/daria/AB_Worker.States` 4 _asab_worker)
      (`|AIMoveTo` (`self.Worker`) (`SceneComponent.K2_GetComponentLocation` (`self.WalkBackPoint`)) null
        (:`OnSuccess`
          (set `/Game/daria/AB_Worker.States` 0 _asab_worker)
          (bind _returnvalue (`GameplayStatics.GetActorOfClass` "/Game/daria/BP_Telega.BP_Telega_C"))
          (`/Game/daria/BP_Telega.TelegaStartMove` _returnvalue))))))

(fn `CalculateInclineAngle`
  (bind (_origin _boxextent) (`KismetSystemLibrary.GetComponentBounds` (`/Game/daria/BP_Telega.Telega` (`self.Telega`))))
  (bind _asab_worker (cast `/Game/daria/AB_Worker` (`SkeletalMeshComponent.GetAnimInstance` (`Character.Mesh` (`self.Worker`)))))
  (set `/Game/daria/AB_Worker.InclineAngle` (/ (- (.z (`SceneComponent.GetSocketLocation` (`Character.Mesh` (`self.Worker`)) "spine_02")) (+ (.z _origin) (/ (.z _boxextent) 2.0))) (`self.InclineAngleMultiplier`)) _asab_worker))

(fn `UserConstructionScript`)