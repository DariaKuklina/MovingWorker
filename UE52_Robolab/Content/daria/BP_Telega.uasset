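; Telega (cart) actor that travels one spline per move, starting when the player pawn's Z-input dispatcher fires its start-move event.
; Each move advances cyclically through AllSplines, snap-attaches to that spline, and uses a timeline to place the Telega mesh along it.
; During travel the anim blueprint's Speed follows physics velocity.
; On arrival it zeroes Speed and calls DoThings on the AllCallable entry with the same index.
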(event `self.ReceiveBeginPlay`
  (`|ExecutionSequence`
    (:`then_0`
      (add `self.TelegaStartMove` (delegate `TelegaStartMove_Event`)))
    (:`then_1`
      (bind _asbp_player_pawn (cast `/Game/Player/BP_PlayerPawn` (`GameplayStatics.GetPlayerCharacter` 0)))
      (add `/Game/Player/BP_PlayerPawn.PlayerInputZ` _asbp_player_pawn (delegate `PlayerInputZ_Event`)))))

(event `TelegaStartMove_Event`
  (bind _currentsplineindex (`self.CurrentSplineIndex`))
  (bind _telega (`self.Telega`))
  (bind _spline (`/Game/daria/BP_Spline.Spline` (`|GetArrayItem` (`self.AllSplines`) _currentsplineindex)))
  (if (not (!= (+ (`self.CurrentSplineIndex`) 1) (`KismetArrayLibrary.Array_Length` (`self.AllSplines`))))
    (set `self.CurrentSplineIndex` -1))
  (bind _result (`/Engine/EditorBlueprintResources/StandardMacros.IncrementInt` _currentsplineindex)
    (:`  `
      (set `self.CurrentSplineIndex` _result)
      (`self.K2_AttachToComponent` _spline "None" "SnapToTarget" "SnapToTarget" "KeepRelative")
      (bind (_direction _speed) (`Timeline|TelegaMoveTimeline` :!via `PlayFromStart`)
        (:`Update`
          (bind _astelega_skeleton_anim_blueprint (cast `/Game/Assets_Telega/telega_Skeleton_AnimBlueprint` (`SkeletalMeshComponent.GetAnimInstance` (`self.Telega`))))
          (bind _returnvalue (`PrimitiveComponent.GetPhysicsLinearVelocity` _telega "None"))
          (set `/Game/Assets_Telega/telega_Skeleton_AnimBlueprint.Speed` (/ (`KismetMathLibrary.VSize` _returnvalue) 60.0) _astelega_skeleton_anim_blueprint)
          (set `/Game/Assets_Telega/telega_Skeleton_AnimBlueprint.Yaw` 0.0 _astelega_skeleton_anim_blueprint)
          (`SceneComponent.K2_SetRelativeTransform` _telega (`SplineComponent.GetTransformAtTime` _spline _speed "Local" false false) false false))
        (:`Finished`
          (set `/Game/Assets_Telega/telega_Skeleton_AnimBlueprint.Speed` 0.0 _astelega_skeleton_anim_blueprint)
          (message `/Game/daria/BPI_Callable.CallDoThings` (`|GetArrayItem` (`self.AllCallable`) (`self.CurrentSplineIndex`)))
          (`KismetSystemLibrary.PrintString` "Telega calls do things"))))))

(event `PlayerInputZ_Event`
  (`self.TelegaStartMove`))

(fn `UserConstructionScript`)